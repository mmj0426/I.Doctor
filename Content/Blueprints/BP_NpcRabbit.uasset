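; BP_NpcRabbit is a rabbit NPC that shows a talk prompt when the player character comes near.
; Overlap events on its Interaction component cast to BP_IDCharacter and set that character's IsOverlapped flag on entry, clearing it on exit.
; On entry it also sets the character's interaction widget text to "대화하기" (Talk) and shows the widget component, then hides it on exit.
; The dialogue itself is not handled in this Blueprint.
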(event `self.Interaction.OnComponentBeginOverlap`
  (params (OverlappedComponent :type "PrimitiveComponent Object Reference") (OtherActor :type "Actor Object Reference") (OtherComp :type "PrimitiveComponent Object Reference") (OtherBodyIndex :type Integer) (bFromSweep :type Boolean) (SweepResult :type "HitResult Structure (by ref)"))
  (bind _asbp_idcharacter (cast `/Game/Blueprints/BP_IDCharacter` OtherActor))
  (bind _output_get (set `self.PlayerCharacter` _asbp_idcharacter))
  (set `/Game/Blueprints/BP_IDCharacter.isOverlapped` true _output_get)
  (bind _widget_interaction (`/Game/Blueprints/BP_IDCharacter.Widget_Interaction` _output_get))
  (bind _asbpwidget_interaction (cast `/Game/Blueprints/UMG/BPWidget_Interaction` (`WidgetComponent.GetUserWidgetObject` _widget_interaction)))
  (set `/Game/Blueprints/UMG/BPWidget_Interaction.Interaction_Text` "대화하기" _asbpwidget_interaction)
  (`SceneComponent.SetVisibility` _widget_interaction true true))

(event `self.Interaction.OnComponentEndOverlap`
  (params (OverlappedComponent :type "PrimitiveComponent Object Reference") (OtherActor :type "Actor Object Reference") (OtherComp :type "PrimitiveComponent Object Reference") (OtherBodyIndex :type Integer))
  (bind _asbp_idcharacter (cast `/Game/Blueprints/BP_IDCharacter` OtherActor))
  (set `/Game/Blueprints/BP_IDCharacter.isOverlapped` false _asbp_idcharacter)
  (`SceneComponent.SetVisibility` (`/Game/Blueprints/BP_IDCharacter.Widget_Interaction` _asbp_idcharacter) false false))

(fn `UserConstructionScript`)
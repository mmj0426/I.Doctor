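; BP_IDCharacter is a character Blueprint that runs NPC dialogue through a Behavior Tree on a spawned dialogue AI controller.
; NpcDialogue shortens the camera boom, opens the dialogue widget in UI-only input, runs the hard-coded rabbit tree and passes the widget through the Blackboard.
; The widget's exit event restores camera and game input, shows an item widget, stops the tree and clears the dialogue widget.
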(event `self.ReceiveBeginPlay`
  (bind _returnvalue (`|SpawnActorFromClass` "/Game/Blueprints/Dialogue/BP_AIController_Dialogue.BP_AIController_Dialogue_C" (`KismetMathLibrary.MakeTransform` (0.0 0.0 0.0)) "Undefined" "OverrideRootScale" null null))
  (set `self.AIController` _returnvalue))

(event `self.NpcDialogue`
  (bind _returnvalue (`GameplayStatics.GetPlayerController` 0))
  (bind _aicontroller (`self.AIController`))
  (`/Engine/EditorBlueprintResources/StandardMacros.IsValid` (`self.DialogueWIdget`)
    (:`Is Not Valid`
      (`|ExecutionSequence`
        (:`then_0`
          (set `SpringArmComponent.TargetArmLength` 300.0 (`self.SpringArm`)))
        (:`then_1`
          (set `self.DialogueTree` "/Game/Blueprints/Dialogue/Rabbit/BT_Dialogue_Rabbit_1.BT_Dialogue_Rabbit_1"))
        (:`then_2`
          (bind _returnvalue_2 (`|CreateWidget` "/Game/Blueprints/UMG/BPWidget_Dialogue.BPWidget_Dialogue_C" _returnvalue))
          (bind _output_get (set `self.DialogueWidget` _returnvalue_2))
          (add `/Game/Blueprints/UMG/BPWidget_Dialogue.OnExit` _output_get (delegate `OnExit_Event_0`))
          (add `/Game/Blueprints/UMG/BPWidget_Dialogue.OnExit` _output_get (delegate `OnExit_Event_0`))
          (`UserWidget.AddToViewport` _output_get 0)
          (`WidgetBlueprintLibrary.SetInputMode_UIOnlyEx` _returnvalue _output_get)
          (set `PlayerController.bShowMouseCursor` true _returnvalue)
          (`AIController.RunBehaviorTree` _aicontroller (`self.DialogueTree`))
          (bind _blackboardcomponent (`AIController.UseBlackboard` _aicontroller "/Game/Blueprints/Dialogue/BB_Dialogue.BB_Dialogue"))
          (`BlackboardComponent.SetValueAsObject` _blackboardcomponent "DialogueWidget" (`self.DialogueWIdget`)))))))

(event `OnExit_Event_0`
  (bind _returnvalue (`Widget.GetOwningPlayer` (`self.DialogueWIdget`)))
  (`WidgetBlueprintLibrary.SetInputMode_GameOnly` _returnvalue)
  (set `PlayerController.bShowMouseCursor` false _returnvalue)
  (set `SpringArmComponent.TargetArmLength` 600.0 (`self.SpringArm`))
  (bind _returnvalue_2 (`|CreateWidget` "/Game/Blueprints/UMG/BPWidget_Item.BPWidget_Item_C" (`GameplayStatics.GetPlayerController` 0)))
  (`UserWidget.AddToViewport` _returnvalue_2 0)
  (`BrainComponent.StopLogic` (`AIController.BrainComponent` (`self.AIController`)) "Dialogue Exited")
  (`Widget.RemoveFromParent` (`self.DialogueWIdget`))
  (set `self.DialogueWIdget` null))

(fn `UserConstructionScript`)
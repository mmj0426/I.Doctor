(event `self.ReceiveBeginPlay`
  (bind _returnvalue (`|SpawnActorFromClass` "/Game/Blueprints/BP_AIController_Dialogue.BP_AIController_Dialogue_C" (`KismetMathLibrary.MakeTransform` (0.0 0.0 0.0)) "Undefined" "OverrideRootScale" null null))
  (set `self.AIController` _returnvalue))

(event `self.NpcDialogue`
  (bind _returnvalue (`GameplayStatics.GetPlayerController` 0))
  (bind _aicontroller (`self.AIController`))
  (`KismetSystemLibrary.PrintString` "Hello")
  (`/Engine/EditorBlueprintResources/StandardMacros.IsValid` (`self.DialogueWidget`)
    (:`Is Not Valid`
      (`|ExecutionSequence`
        (:`then_1`
          (bind _returnvalue_2 (`|CreateWidget` "/Game/Blueprints/UMG/BPWidget_Dialogue.BPWidget_Dialogue_C" _returnvalue))
          (bind _output_get (set `self.DialogueWidget` _returnvalue_2))
          (add `/Game/Blueprints/UMG/BPWidget_Dialogue.OnExit` _output_get (delegate `OnExit_Event_0`))
          (add `/Game/Blueprints/UMG/BPWidget_Dialogue.OnExit` _output_get (delegate `OnExit_Event_0`))
          (`UserWidget.AddToViewport` _output_get 0)
          (`WidgetBlueprintLibrary.SetInputMode_UIOnlyEx` _returnvalue _output_get)
          (set `PlayerController.bShowMouseCursor` true _returnvalue)
          (`AIController.RunBehaviorTree` _aicontroller (`self.DialoigueTree`))
          (bind _blackboardcomponent (`AIController.UseBlackboard` _aicontroller "/Game/Blueprints/BB_Dialogue.BB_Dialogue"))
          (`BlackboardComponent.SetValueAsObject` _blackboardcomponent "DialogueWidget" (`self.DialogueWidget`)))))))

(event `OnExit_Event_0`
  (bind _returnvalue (`Widget.GetOwningPlayer` (`self.DialogueWidget`)))
  (`WidgetBlueprintLibrary.SetInputMode_GameOnly` _returnvalue)
  (set `PlayerController.bShowMouseCursor` false _returnvalue)
  (`BrainComponent.StopLogic` (`AIController.BrainComponent` (`self.AIController`)) "Dialogue Exited")
  (`Widget.RemoveFromParent` (`self.DialogueWidget`))
  (set `self.DialogueWidget` null))

(fn `UserConstructionScript`)